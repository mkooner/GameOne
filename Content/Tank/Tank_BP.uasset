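; Player-controllable tank Blueprint that drives on two tracks, aims and fires, and collects coins as points.
; BeginPlay wires barrel and turret into TankAiming, both tracks into TankMovement, and itself into the health bar widget.
; Input drives movement through TankMovement or per-track throttles, fires through TankAiming, orbits a gimbal and spring-arm camera, and toggles first-person view.
; Overlapping a Coin increments and prints Points.
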(event `self.ReceiveBeginPlay`
  (`TankAimComponent.Initialize` (`self.Tank Aiming`) (`self.TankBarrel`) (`self.TankTurret`))
  (`TankMovementComponent.Initialize` (`self.TankMovement`) (`self.TrackL`) (`self.TrackR`))
  (bind _ashealth_bar (cast `/Game/UI/HealthBar` (`WidgetComponent.GetUserWidgetObject` (`self.Widget`))))
  (set `/Game/UI/HealthBar.Tank` self _ashealth_bar))

(event `self.ReceiveActorBeginOverlap`
  (params (OtherActor :type "Actor Object Reference"))
  (cast `/Game/Coin` OtherActor)
  (bind _output_get (set `self.Points` (+ (`self.Points`) 1)))
  (`KismetSystemLibrary.PrintString` (`KismetStringLibrary.Conv_IntToString` _output_get)))

(event `self.ReceiveTick`
  (params (DeltaSeconds :type "Float (single-precision)")))

(event `InputAxis|AimAzmuth`
  (params (AxisValue :type "Float (single-precision)"))
  ;[1 1 1] Camera Controls
  (`SceneComponent.K2_AddLocalRotation` (`self.Azimuth Gimbal`) (`KismetMathLibrary.MakeRotator` 0.0 0.0 (* AxisValue (`GameplayStatics.GetWorldDeltaSeconds`) 100.0)) false false))

(event `InputAxis|AimElevation`
  (params (AxisValue :type "Float (single-precision)"))
  ;[1 1 1] Camera Controls
  (`SceneComponent.K2_AddLocalRotation` (`self.SpringArm`) (`KismetMathLibrary.MakeRotator` 0.0 (* AxisValue (`GameplayStatics.GetWorldDeltaSeconds`) 100.0)) false false))

(event `InputAxis|Move`
  (params (AxisValue :type "Float (single-precision)"))
  ;[1 1 1] Movement Binding Input
  (`TankMovementComponent.MoveFoward` (`self.TankMovement`) AxisValue))

(event `InputAction|Fire`
  (params (Key :type "Key Structure" :default "AnyKey"))
  ;[1 1 1] Throttle Input Binding
  (:`Pressed`
    (`TankAimComponent.Fire` (`self.Tank Aiming`))))

(event `InputAxis|Turn`
  (params (AxisValue :type "Float (single-precision)"))
  ;[1 1 1] Movement Binding Input
  (`TankMovementComponent.MoveTurn` (`self.TankMovement`) AxisValue))

(event `InputAxis|Left Track Throttle`
  (params (AxisValue :type "Float (single-precision)"))
  ;[1 1 1] Throttle Input Binding
  (`TankTrack.SetThrottle` (`self.TrackL`) AxisValue))

(event `InputAction|Camera`
  (params (Key :type "Key Structure" :default "AnyKey"))
  ;[1 1 1] Movement Binding Input
  (:`Pressed`
    (`ActorComponent.ToggleActive` (`self.FirstPerson`))
    (`ActorComponent.ToggleActive` (`self.Camera`))))

(event `InputAxis|Right Track Throttle`
  (params (AxisValue :type "Float (single-precision)"))
  ;[1 1 1] Throttle Input Binding
  (`TankTrack.SetThrottle` (`self.TrackR`) AxisValue))

(fn `UserConstructionScript`)